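; Main level game mode that builds a triangular pyramid of BP_Tile actors and links them into a diagonal neighbour grid.
; BeginPlay spawns LayerLevel staggered rows in the XZ plane, each one tile wider than the last, storing them in TilesArray.
; ConnetTiles then walks that flat array with running row counters, using index offsets to set each tile's Up, Down, Left and Right references, skipping those beyond the edges.
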(event `self.ReceiveBeginPlay`
  (`|ExecutionSequence`
    (:`then_0`
      ;[1 1 1] Create Tiles
      (for _index (range (`self.LayerLevel`))
        (for _index_2 (range (+ _index 1))
          (bind _returnvalue (`|SpawnActorFromClass` "/Game/BluePrint/BP_Tile.BP_Tile_C" (`KismetMathLibrary.MakeTransform` (`KismetMathLibrary.MakeVector` (+ (* _index_2 32.0) (* _index -16.0)) 5.0 (* _index -24.0))) "Undefined" "OverrideRootScale" null null))
          (`KismetArrayLibrary.Array_Add` (`self.TilesArray`) _returnvalue))))
    (:`then_1`
      ;[1 1 1] Connet TIles
      (`self.ConnetTiles`))))

(fn `ConnetTiles`
  (locals (LayerLevelCount :type Integer :default 1) (LayerFirstIdx :type Integer) (LayerEndIdx :type Integer))
  (for (_array_element _array_index) (`self.TilesArray`)
    (`|ExecutionSequence`
      (:`then_0`
        ;[1 1 1] If it is not last row
        (if (!= (`local.LayerLevelCount`) (`self.LayerLevel`))
          (`|ExecutionSequence`
            (:`then_0`
              ;[1 1 1] Set DownTile
              (set `/Game/BluePrint/BP_Tile.DownTile` (`|GetArrayItem` (`self.TilesArray`) (+ _array_index (`local.LayerLevelCount`))) _array_element))
            (:`then_1`
              ;[1 1 1] Set RightTile
              (set `/Game/BluePrint/BP_Tile.RightTile` (`|GetArrayItem` (`self.TilesArray`) (+ _array_index (+ (`local.LayerLevelCount`) 1))) _array_element)))))
      (:`then_1`
        ;[1 1 1] If it is not first row
        (if (!= (`local.LayerLevelCount`) 1)
          (`|ExecutionSequence`
            (:`then_0`
              ;[1 1 1] Check if it is first tile in layer
              (if (== _array_index (`local.LayerFirstIdx`))
                ;[1 1 1] Set UpTile
                (set `/Game/BluePrint/BP_Tile.UpTile` (`|GetArrayItem` (`self.TilesArray`) (- _array_index (- (`local.LayerLevelCount`) 1))) _array_element :!label _label)
                (else
                  ;[1 1 1] Set LeftTile
                  (set `/Game/BluePrint/BP_Tile.LeftTile` (`|GetArrayItem` (`self.TilesArray`) (- _array_index (`local.LayerLevelCount`))) _array_element :!label _label_2))))
            (:`then_1`
              ;[1 1 1] Check if it is last tile in layer
              (if (== _array_index (`local.LayerEndIdx`))
                (goto _label_2)
                (else
                  (goto _label)))))))
      (:`then_2`
        ;[1 1 1] Increase LayerLevelCount, Set Layer First Idx, Last Idx
        (if (== _array_index (`local.LayerEndIdx`))
          (`/Engine/EditorBlueprintResources/StandardMacros.IncrementInt` (`local.LayerLevelCount`)
            (:`  `
              (set `local.LayerFirstIdx` (+ (`local.LayerEndIdx`) 1))
              (set `local.LayerEndIdx` (+ (`local.LayerFirstIdx`) (- (`local.LayerLevelCount`) 1))))))))))

(fn `UserConstructionScript`)