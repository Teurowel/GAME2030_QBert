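; Game instance that owns the game's persistent top-10 leaderboard of initials and scores.
; On Init it loads the BP_SaveGame slot, or creates one seeded with ten placeholder entries.
; CheckTop10Score returns the first rank a score strictly beats.
; AddNewHighScore drops the last entry, inserts the new one at the given index, then copies the board to the save object and writes it to the slot.
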(event `self.ReceiveInit`
  (bind _returnvalue (`GameplayStatics.LoadGameFromSlot` "LeaderBoardData"))
  (`/Engine/EditorBlueprintResources/StandardMacros.IsValid` _returnvalue
    (:`Is Valid`
      (`KismetSystemLibrary.PrintString` "Load Save Game")
      (bind _asbp_save_game (cast `/Game/BluePrint/BP_SaveGame` _returnvalue))
      (bind _output_get (set `self.SaveGame` _asbp_save_game))
      (set `self.LeaderBoard` (`/Game/BluePrint/BP_SaveGame.LeaderBoard` _output_get)))
    (:`Is Not Valid`
      (`KismetSystemLibrary.PrintString` "Create New Save Game")
      ;[1 1 1] Create New Save Game
      (bind _returnvalue_2 (`GameplayStatics.CreateSaveGameObject` "/Game/BluePrint/BP_SaveGame.BP_SaveGame_C"))
      (set `self.SaveGame` _returnvalue_2)
      ;[1 1 1] Init LeaderBoard
      (for _ (range 10)
        (`KismetArrayLibrary.Array_Add` (`self.LeaderBoard`) (make `/Game/BluePrint/Struct_LeaderBoard` "AAA"))
        ;[1 1 1] Copy the Data
        (`/Game/BluePrint/BP_SaveGame.CopyLeaderBoard` (`self.SaveGame`) (`self.LeaderBoard`))
        ;[1 1 1] Save To Slot
        (`GameplayStatics.SaveGameToSlot` (`self.SaveGame`) "LeaderBoardData")))))

(fn `AddNewHighScore`
  (params (Idx :type Integer) (NewHighScore :type "/Game/BluePrint/Struct_LeaderBoard Structure"))
  (bind _leaderboard (`self.LeaderBoard`))
  (`KismetArrayLibrary.Array_Remove` _leaderboard (- (`KismetArrayLibrary.Array_Length` _leaderboard) 1))
  (`KismetArrayLibrary.Array_Insert` (`self.LeaderBoard`) NewHighScore Idx)
  ;[1 1 1] Copy the Data
  (`/Game/BluePrint/BP_SaveGame.CopyLeaderBoard` (`self.SaveGame`) (`self.LeaderBoard`))
  ;[1 1 1] Save To Slot
  (`GameplayStatics.SaveGameToSlot` (`self.SaveGame`) "LeaderBoardData"))

(fn `CheckTop10Score`
  (params (Score :type Integer))
  (returns (Result :type Boolean) (Idx :type Integer))
  (for (_array_element _array_index) (`self.LeaderBoard`)
    (if (> Score (`.Score_5_27DF9ED04AF96667CC548E969D01733E` (break `/Game/BluePrint/Struct_LeaderBoard` _array_element)))
      (return true _array_index)))
  (return false 0))