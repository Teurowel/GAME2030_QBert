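; Spawner actor that periodically drops red and green ball enemies onto the level's tiles.
; BeginPlay starts two independent timers, a randomized one for red balls and a fixed, shorter one for green balls.
; Each timer event picks one of two tiles from GM_MainLevel's TilesArray, spawns the ball above it with that tile as CurrentTile, then re-arms its own timer.
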(event `self.ReceiveBeginPlay`
  ;[1 1 1] Set Timer For Creating Red Ball
  (bind _returnvalue (`KismetSystemLibrary.K2_SetTimer` null "CreateRedBall" (`KismetMathLibrary.RandomFloatInRange` 5.0 7.0)))
  (set `self.CreateRedBallTimer` _returnvalue)
  (bind _returnvalue_2 (`KismetSystemLibrary.K2_SetTimer` null "CreateGreenBall" 2.0))
  (set `self.CreateGreenBallTimer` _returnvalue_2))

(event `CreateRedBall`
  (bind (_returnvalue_x _returnvalue_y _returnvalue_z) (`KismetMathLibrary.BreakVector` (`self.K2_GetActorLocation` (`self.SelectedTile`))))
  ;[1 1 1] Randomly Select Spawn Tile
  (set `self.SelectedTile` (`|GetArrayItem` (`/Game/GameMode/GM_MainLevel.TilesArray` (cast `/Game/GameMode/GM_MainLevel` (`GameplayStatics.GetGameMode`) :!pure true)) (`KismetMathLibrary.RandomIntegerInRange` 1 2)))
  ;[1 1 1] Spawn Enemy
  (`|SpawnActorFromClass` "/Game/BluePrint/BP_RedBall.BP_RedBall_C" (`KismetMathLibrary.MakeTransform` (`KismetMathLibrary.MakeVector` _returnvalue_x 5.2 (+ _returnvalue_z 100.0))) "Undefined" "OverrideRootScale" null (`self.SelectedTile`) null)
  ;[1 1 1] Reset Timer
  (`KismetSystemLibrary.K2_ClearAndInvalidateTimerHandle` (`self.CreateRedBallTimer`))
  (bind _returnvalue (`KismetSystemLibrary.K2_SetTimer` null "CreateRedBall" (`KismetMathLibrary.RandomFloatInRange` 5.0 7.0)))
  (set `self.CreateRedBallTimer` _returnvalue))

(event `CreateGreenBall`
  (bind (_returnvalue_x _returnvalue_y _returnvalue_z) (`KismetMathLibrary.BreakVector` (`self.K2_GetActorLocation` (`self.SelectedTile`))))
  ;[1 1 1] Randomly Select Spawn Tile
  (set `self.SelectedTile` (`|GetArrayItem` (`/Game/GameMode/GM_MainLevel.TilesArray` (cast `/Game/GameMode/GM_MainLevel` (`GameplayStatics.GetGameMode`) :!pure true)) (`KismetMathLibrary.RandomIntegerInRange` 1 2)))
  ;[1 1 1] Spawn Enemy
  (`|SpawnActorFromClass` "/Game/BluePrint/BP_GreenBall.BP_GreenBall_C" (`KismetMathLibrary.MakeTransform` (`KismetMathLibrary.MakeVector` _returnvalue_x 5.2 (+ _returnvalue_z 100.0))) "Undefined" "OverrideRootScale" null (`self.SelectedTile`) null)
  ;[1 1 1] Reset Timer
  (`KismetSystemLibrary.K2_ClearAndInvalidateTimerHandle` (`self.CreateGreenBallTimer`))
  (bind _returnvalue (`KismetSystemLibrary.K2_SetTimer` null "CreateGreenBall" 2.0))
  (set `self.CreateGreenBallTimer` _returnvalue))

(fn `UserConstructionScript`)