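; Coily enemy for a Q*bert-style game that, once activated, hops randomly down the tiles, then chases Qbert.
; Looping timers drive each hop, switching to chase mode when the chosen downward tile is missing.
; Chase steps compare positions with Qbert or his elevator location to pick a neighbouring tile and flipbook.
; Timelines move it along a repositioned spline arc; chasing an elevator off an upper edge makes it fall, notifying GM_MainLevel of its defeat.
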(event `self.ReceiveTick`
  (params (DeltaSeconds :type "Float (single-precision)"))
  ;[1 1 1] Once Activated, Start Moving
  (if (`self.Activate`)
    (`/Engine/EditorBlueprintResources/StandardMacros.DoOnce` false
      (:`Completed`
        (bind _returnvalue (`KismetSystemLibrary.K2_SetTimer` null "MoveAlongSpline" (`self.MoveSpeed`) true))
        (set `self.MoveAlongSplineTimer` _returnvalue)))))

(event `MoveAlongSpline`
  ;[1 1 1] Randomly Select a tile Where red ball will move to
  (`GameplayStatics.PlaySound2D` "/Game/Sound/BallJumpSound_Cue.BallJumpSound_Cue" 1.0 1.0 0.0 null null)
  (if (== (`KismetMathLibrary.RandomIntegerInRange` 0 1) 0)
    (`/Engine/EditorBlueprintResources/StandardMacros.IsValid` (`/Game/BluePrint/BP_Tile.RightTile` (`self.CurrentTile`))
      (:`Is Valid`
        (set `self.CurrentTile` (`/Game/BluePrint/BP_Tile.RightTile` (`self.CurrentTile`)))
        ;[1 1 1] Move along Spline
        (`self.K2_SetActorLocation` (`self.JumpArcSpline`) (`self.K2_GetActorLocation`) false false :!label _label)
        (`SplineComponent.SetLocationAtSplinePoint` (`/Game/BluePrint/BP_QbertJumpArcSpline.Spline` (`self.JumpArcSpline`)) 1 (+ (`self.K2_GetActorLocation` (`self.CurrentTile`)) (0.0 0.2 40.0)) "World" false)
        (`SplineComponent.SetLocationAtSplinePoint` (`/Game/BluePrint/BP_QbertJumpArcSpline.Spline` (`self.JumpArcSpline`)) 2 (+ (`self.K2_GetActorLocation` (`self.CurrentTile`)) (0.0 0.2 10.0)) "World" true)
        (bind (_direction _0_1) (`Timeline|Timeline_1` :!via `PlayFromStart`)
          (:`Update`
            (`self.K2_SetActorLocation` (`SplineComponent.GetLocationAtDistanceAlongSpline` (`/Game/BluePrint/BP_QbertJumpArcSpline.Spline` (`self.JumpArcSpline`)) (`KismetMathLibrary.Lerp` 0.0 (`SplineComponent.GetSplineLength` (`/Game/BluePrint/BP_QbertJumpArcSpline.Spline` (`self.JumpArcSpline`))) _0_1) "World")))))
      (:`Is Not Valid`
        (`KismetSystemLibrary.K2_ClearAndInvalidateTimerHandle` (`self.MoveAlongSplineTimer`))
        (`SceneComponent.K2_AddLocalOffset` (`self.PaperFlipbook`) (0.0 0.0 0.0) false false)
        (`SceneComponent.K2_AddLocalOffset` (`self.Box`) (0.0 0.0 -10.0) false false)
        (bind _returnvalue (`KismetSystemLibrary.K2_SetTimer` null "ChaseQbertWithSpline" (`self.MoveSpeed`) true))
        (set `self.MoveAlongSplineTimer` _returnvalue)))
    (else
      (`/Engine/EditorBlueprintResources/StandardMacros.IsValid` (`/Game/BluePrint/BP_Tile.DownTile` (`self.CurrentTile`))
        (:`Is Valid`
          (set `self.CurrentTile` (`/Game/BluePrint/BP_Tile.DownTile` (`self.CurrentTile`)))
          (goto _label))
        (:`Is Not Valid`
          (`KismetSystemLibrary.K2_ClearAndInvalidateTimerHandle` (`self.MoveAlongSplineTimer`))
          (`SceneComponent.K2_AddLocalOffset` (`self.PaperFlipbook`) (0.0 0.0 0.0) false false)
          (`SceneComponent.K2_AddLocalOffset` (`self.Box`) (0.0 0.0 -10.0) false false)
          (bind _returnvalue_2 (`KismetSystemLibrary.K2_SetTimer` null "ChaseQbertWithSpline" (`self.MoveSpeed`) true))
          (set `self.MoveAlongSplineTimer` _returnvalue_2))))))

(event `MoveAlongFallSpline`
  (bind _movealongsplinetimer (`self.MoveAlongSplineTimer`))
  ;[1 1 1] Move along Fall Spline
  (`|ExecutionSequence`
    (:`then_0`
      (if (`KismetSystemLibrary.K2_IsValidTimerHandle` _movealongsplinetimer)
        (`KismetSystemLibrary.K2_ClearAndInvalidateTimerHandle` _movealongsplinetimer)))
    (:`then_1`
      (`self.K2_SetActorLocation` (`self.JumpArcSpline`) (`self.K2_GetActorLocation`) false false)
      (`SplineComponent.SetLocationAtSplinePoint` (`/Game/BluePrint/BP_QbertJumpArcSpline.Spline` (`self.JumpArcSpline`)) 1 (+ (`self.FallTileLocation`) (0.0 -2.0 40.0)) "World" false)
      (`SplineComponent.SetLocationAtSplinePoint` (`/Game/BluePrint/BP_QbertJumpArcSpline.Spline` (`self.JumpArcSpline`)) 2 (+ (`self.FallTileLocation`) (0.0 -2.0 -100.0)) "World" true)
      (bind (_direction _0_1) (`Timeline|Timeline_2` :!via `PlayFromStart`)
        (:`Update`
          (`self.K2_SetActorLocation` (`SplineComponent.GetLocationAtDistanceAlongSpline` (`/Game/BluePrint/BP_QbertJumpArcSpline.Spline` (`self.JumpArcSpline`)) (`KismetMathLibrary.Lerp` 0.0 (`SplineComponent.GetSplineLength` (`/Game/BluePrint/BP_QbertJumpArcSpline.Spline` (`self.JumpArcSpline`))) _0_1) "World")))
        (:`Finished`
          (`/Game/GameMode/GM_MainLevel.DefeatedCoily` (cast `/Game/GameMode/GM_MainLevel` (`GameplayStatics.GetGameMode`) :!pure true)))))))

(event `ChaseQbertWithSpline`
  (bind _returnvalue_x (`KismetMathLibrary.BreakVector` (`self.K2_GetActorLocation` (`self.CurrentTile`))))
  (bind (_returnvalue_x_2 _returnvalue_y _returnvalue_z) (`KismetMathLibrary.BreakVector` (`self.K2_GetActorLocation` (`self.CurrentTile`))))
  (bind _returnvalue_x_3 (`KismetMathLibrary.BreakVector` (`self.K2_GetActorLocation` (`self.CurrentTile`))))
  (bind (_returnvalue_x_4 _returnvalue_y_2 _returnvalue_z_2) (`KismetMathLibrary.BreakVector` (`self.K2_GetActorLocation` (`self.CurrentTile`))))
  (bind _elevatortemplocation_x (`KismetMathLibrary.BreakVector` (`/Game/BluePrint/BP_Qbert.ElevatorTempLocation` (cast `/Game/BluePrint/BP_Qbert` (`GameplayStatics.GetPlayerPawn` 0) :!pure true))))
  (bind (_elevatortemplocation_x_2 _elevatortemplocation_y _elevatortemplocation_z) (`KismetMathLibrary.BreakVector` (`/Game/BluePrint/BP_Qbert.ElevatorTempLocation` (cast `/Game/BluePrint/BP_Qbert` (`GameplayStatics.GetPlayerPawn` 0) :!pure true))))
  (bind (_returnvalue_x_5 _returnvalue_y_3 _returnvalue_z_3) (`KismetMathLibrary.BreakVector` (`self.K2_GetActorLocation` (`/Game/BluePrint/BP_Qbert.CurrentTile` (cast `/Game/BluePrint/BP_Qbert` (`GameplayStatics.GetPlayerPawn` 0) :!pure true)))))
  (bind _returnvalue_x_6 (`KismetMathLibrary.BreakVector` (`self.K2_GetActorLocation` (`/Game/BluePrint/BP_Qbert.CurrentTile` (cast `/Game/BluePrint/BP_Qbert` (`GameplayStatics.GetPlayerPawn` 0) :!pure true)))))
  ;[1 1 1] Coily CHase Qber
  (`GameplayStatics.PlaySound2D` "/Game/Sound/CoilyJumpSound_Cue.CoilyJumpSound_Cue" 1.0 1.0 0.0 null null)
  (if (`/Game/BluePrint/BP_Qbert.IsCurrentTileElevator` (cast `/Game/BluePrint/BP_Qbert` (`GameplayStatics.GetPlayerPawn` 0) :!pure true))
    ;;[1 1 1] When Qbert is on the elevator
    (set `self.GoToLeft` (>= _returnvalue_x_3 _elevatortemplocation_x))
    (set `self.GoToDown` (>= _returnvalue_z _elevatortemplocation_z))
    (else
      ;;[1 1 1] Decide which direction to go, left or right
      (set `self.GoToLeft` (>= _returnvalue_x _returnvalue_x_6))
      ;;[1 1 1] Decide which direction to go, Up or Down
      (set `self.GoToDown` (>= _returnvalue_z_2 _returnvalue_z_3))))
  (if (`self.GoToLeft`)
    (if (`self.GoToDown`)
      (`KismetSystemLibrary.PrintString` "Left Down")
      (`PaperFlipbookComponent.SetFlipbook` (`self.PaperFlipbook`) "/Game/Sprite/Coily/FlipBook_Coily_Down.FlipBook_Coily_Down")
      (`/Engine/EditorBlueprintResources/StandardMacros.IsValid` (`/Game/BluePrint/BP_Tile.DownTile` (`self.CurrentTile`))
        (:`Is Valid`
          (set `self.CurrentTile` (`/Game/BluePrint/BP_Tile.DownTile` (`self.CurrentTile`))))
        (:`Is Not Valid`
          (set `self.CurrentTile` (`/Game/BluePrint/BP_Tile.LeftTile` (`self.CurrentTile`)) :!label _label_2)))
      ;;[1 1 1] Move Along Spline
      (`self.K2_SetActorLocation` (`self.JumpArcSpline`) (`self.K2_GetActorLocation`) false false :!label _label_3)
      (`SplineComponent.SetLocationAtSplinePoint` (`/Game/BluePrint/BP_QbertJumpArcSpline.Spline` (`self.JumpArcSpline`)) 1 (+ (`self.K2_GetActorLocation` (`self.CurrentTile`)) (0.0 0.2 40.0)) "World" false)
      (`SplineComponent.SetLocationAtSplinePoint` (`/Game/BluePrint/BP_QbertJumpArcSpline.Spline` (`self.JumpArcSpline`)) 2 (+ (`self.K2_GetActorLocation` (`self.CurrentTile`)) (0.0 0.2 20.0)) "World" true)
      (bind (_direction _0_1) (`Timeline|Timeline_3` :!via `PlayFromStart`)
        (:`Update`
          (`self.K2_SetActorLocation` (`SplineComponent.GetLocationAtDistanceAlongSpline` (`/Game/BluePrint/BP_QbertJumpArcSpline.Spline` (`self.JumpArcSpline`)) (`KismetMathLibrary.Lerp` 0.0 (`SplineComponent.GetSplineLength` (`/Game/BluePrint/BP_QbertJumpArcSpline.Spline` (`self.JumpArcSpline`))) _0_1) "World"))))
      (else
        (`KismetSystemLibrary.PrintString` "Left Up")
        (`PaperFlipbookComponent.SetFlipbook` (`self.PaperFlipbook`) "/Game/Sprite/Coily/FlipBook_Coily_Left.FlipBook_Coily_Left")
        (`/Engine/EditorBlueprintResources/StandardMacros.IsValid` (`/Game/BluePrint/BP_Tile.LeftTile` (`self.CurrentTile`))
          (:`Is Valid`
            (goto _label_2))
          (:`Is Not Valid`
            (if (`/Game/BluePrint/BP_Qbert.IsCurrentTileElevator` (cast `/Game/BluePrint/BP_Qbert` (`GameplayStatics.GetPlayerPawn` 0) :!pure true))
              (set `self.FallTileLocation` (+ (`self.K2_GetActorLocation` (`self.CurrentTile`)) (-16.0 0.0 -24.0)))
              (`self.MoveAlongFallSpline`))))))
    (elif (`self.GoToDown`)
      (`KismetSystemLibrary.PrintString` "RIght Down")
      (`PaperFlipbookComponent.SetFlipbook` (`self.PaperFlipbook`) "/Game/Sprite/Coily/FlipBook_Coily_Right.FlipBook_Coily_Right")
      (`/Engine/EditorBlueprintResources/StandardMacros.IsValid` (`/Game/BluePrint/BP_Tile.RightTile` (`self.CurrentTile`))
        (:`Is Valid`
          (set `self.CurrentTile` (`/Game/BluePrint/BP_Tile.RightTile` (`self.CurrentTile`)))
          (goto _label_3))
        (:`Is Not Valid`
          (set `self.CurrentTile` (`/Game/BluePrint/BP_Tile.UpTile` (`self.CurrentTile`)) :!label _label_4)
          (goto _label_3)))
      (else
        (`KismetSystemLibrary.PrintString` "Right Up")
        (`PaperFlipbookComponent.SetFlipbook` (`self.PaperFlipbook`) "/Game/Sprite/Coily/FlipBook_Coily_Up.FlipBook_Coily_Up")
        (`/Engine/EditorBlueprintResources/StandardMacros.IsValid` (`/Game/BluePrint/BP_Tile.UpTile` (`self.CurrentTile`))
          (:`Is Valid`
            (goto _label_4))
          (:`Is Not Valid`
            (if (`/Game/BluePrint/BP_Qbert.IsCurrentTileElevator` (cast `/Game/BluePrint/BP_Qbert` (`GameplayStatics.GetPlayerPawn` 0) :!pure true))
              (set `self.FallTileLocation` (+ (`self.K2_GetActorLocation` (`self.CurrentTile`)) (16.0 0.0 -24.0)))
              (`self.MoveAlongFallSpline`))))))))

(fn `UserConstructionScript`
  (`parent.UserConstructionScript`))