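; Player-controlled Q*bert that hops between linked tiles, starting on the first tile in GM_MainLevel's array.
; Directional input, locked during movement, picks the neighbouring tile or a fall point if none exists.
; A spawned BP_QbertJumpArcSpline is reshaped for each move, and timelines move the actor along it.
; Landing calls the tile's ChangeColor; falling resets the player after a delay and decreases lives through the game mode.
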(event `self.ReceiveBeginPlay`
  ;[1 1 1] Set Initial Tile(first one)
  (set `self.CurrentTile` (`|GetArrayItem` (`/Game/GameMode/GM_MainLevel.TilesArray` (cast `/Game/GameMode/GM_MainLevel` (`GameplayStatics.GetGameMode`) :!pure true))))
  ;[1 1 1] Create Jump Arc Spline
  (bind _returnvalue (`|SpawnActorFromClass` "/Game/BluePrint/BP_QbertJumpArcSpline.BP_QbertJumpArcSpline_C" (`KismetMathLibrary.MakeTransform` (0.0 0.0 0.0)) "Undefined" "OverrideRootScale" null null))
  (set `self.JumpArcSpline` _returnvalue))

(event `InputAction|MoveUp`
  (params (Key :type "Key Structure"))
  ;[1 1 1] Input
  ;;[1 1 1] Move Up
  (:`Pressed`
    (if (not (`self.IsMoving`))
      (set `self.IsMoving` true)
      (set `self.MoveUpOrLeft` true)
      (set `self.MoveDownOrRight` false)
      (`/Engine/EditorBlueprintResources/StandardMacros.IsValid` (`/Game/BluePrint/BP_Tile.UpTile` (`self.CurrentTile`))
        (:`Is Valid`
          (set `self.CurrentTile` (`/Game/BluePrint/BP_Tile.UpTile` (`self.CurrentTile`)))
          (`self.MoveAlongSpline`))
        (:`Is Not Valid`
          (set `self.FallTileLocation` (+ (`self.K2_GetActorLocation` (`self.CurrentTile`)) (16.0 0.0 24.0)))
          (`self.MoveAlongFallSpline`))))))

(event `InputAction|MoveRight`
  (params (Key :type "Key Structure"))
  ;[1 1 1] Input
  ;;[1 1 1] Move Right
  (:`Pressed`
    (if (not (`self.IsMoving`))
      (set `self.IsMoving` true)
      (set `self.MoveUpOrLeft` false)
      (set `self.MoveDownOrRight` true)
      (`/Engine/EditorBlueprintResources/StandardMacros.IsValid` (`/Game/BluePrint/BP_Tile.RightTile` (`self.CurrentTile`))
        (:`Is Valid`
          (set `self.CurrentTile` (`/Game/BluePrint/BP_Tile.RightTile` (`self.CurrentTile`)))
          (`self.MoveAlongSpline`))
        (:`Is Not Valid`
          (set `self.FallTileLocation` (+ (`self.K2_GetActorLocation` (`self.CurrentTile`)) (16.0 0.0 -24.0)))
          (`self.MoveAlongFallSpline`))))))

(event `InputAction|MoveLeft`
  (params (Key :type "Key Structure"))
  ;[1 1 1] Input
  ;;[1 1 1] Move Left
  (:`Pressed`
    (if (not (`self.IsMoving`))
      (set `self.IsMoving` true)
      (set `self.MoveUpOrLeft` true)
      (set `self.MoveDownOrRight` false)
      (`/Engine/EditorBlueprintResources/StandardMacros.IsValid` (`/Game/BluePrint/BP_Tile.LeftTile` (`self.CurrentTile`))
        (:`Is Valid`
          (set `self.CurrentTile` (`/Game/BluePrint/BP_Tile.LeftTile` (`self.CurrentTile`)))
          (`self.MoveAlongSpline`))
        (:`Is Not Valid`
          (set `self.FallTileLocation` (+ (`self.K2_GetActorLocation` (`self.CurrentTile`)) (-16.0 0.0 24.0)))
          (`self.MoveAlongFallSpline`))))))

(event `InputAction|MoveDown`
  (params (Key :type "Key Structure"))
  ;[1 1 1] Input
  ;;[1 1 1] Move DOwn
  (:`Pressed`
    (if (not (`self.IsMoving`))
      (set `self.IsMoving` true)
      (set `self.MoveUpOrLeft` false)
      (set `self.MoveDownOrRight` true)
      (`/Engine/EditorBlueprintResources/StandardMacros.IsValid` (`/Game/BluePrint/BP_Tile.DownTile` (`self.CurrentTile`))
        (:`Is Valid`
          (set `self.CurrentTile` (`/Game/BluePrint/BP_Tile.DownTile` (`self.CurrentTile`)))
          (`self.MoveAlongSpline`))
        (:`Is Not Valid`
          (set `self.FallTileLocation` (+ (`self.K2_GetActorLocation` (`self.CurrentTile`)) (-16.0 0.0 -24.0)))
          (`self.MoveAlongFallSpline`))))))

(event `MoveAlongSpline`
  ;[1 1 1] Move Along Spline
  (`self.K2_SetActorLocation` (`self.JumpArcSpline`) (`self.K2_GetActorLocation`) false false)
  (if (`self.MoveDownOrRight`)
    (`SplineComponent.SetLocationAtSplinePoint` (`/Game/BluePrint/BP_QbertJumpArcSpline.Spline` (`self.JumpArcSpline`)) 1 (+ (`self.K2_GetActorLocation` (`self.CurrentTile`)) (0.0 0.2 40.0)) "World" true)
    (else
      (`SplineComponent.SetLocationAtSplinePoint` (`/Game/BluePrint/BP_QbertJumpArcSpline.Spline` (`self.JumpArcSpline`)) 1 (+ (`self.K2_GetActorLocation`) (0.0 0.2 25.0)) "World" true)))
  (`SplineComponent.SetLocationAtSplinePoint` (`/Game/BluePrint/BP_QbertJumpArcSpline.Spline` (`self.JumpArcSpline`)) 2 (+ (`self.K2_GetActorLocation` (`self.CurrentTile`)) (0.0 0.2 16.0)) "World" true)
  (bind (_direction _0_1) (`Timeline|Timeline_0` :!via `PlayFromStart`)
    (:`Update`
      (`self.K2_SetActorLocation` (`SplineComponent.GetLocationAtDistanceAlongSpline` (`/Game/BluePrint/BP_QbertJumpArcSpline.Spline` (`self.JumpArcSpline`)) (`KismetMathLibrary.Lerp` 0.0 (`SplineComponent.GetSplineLength` (`/Game/BluePrint/BP_QbertJumpArcSpline.Spline` (`self.JumpArcSpline`))) _0_1) "World")))
    (:`Finished`
      (set `self.IsMoving` false)
      (`/Game/BluePrint/BP_Tile.ChangeColor` (`self.CurrentTile`)))))

(event `MoveAlongFallSpline`
  ;[1 1 1] Move Along Fall Spline
  (`self.K2_SetActorLocation` (`self.JumpArcSpline`) (`self.K2_GetActorLocation`) false false)
  (if (`self.MoveDownOrRight`)
    (`SplineComponent.SetLocationAtSplinePoint` (`/Game/BluePrint/BP_QbertJumpArcSpline.Spline` (`self.JumpArcSpline`)) 1 (+ (`self.FallTileLocation`) (0.0 2.0 20.0)) "World" true)
    (else
      (`SplineComponent.SetLocationAtSplinePoint` (`/Game/BluePrint/BP_QbertJumpArcSpline.Spline` (`self.JumpArcSpline`)) 1 (+ (`self.FallTileLocation`) (0.0 -2.0 5.0)) "World" true)))
  (`SplineComponent.SetLocationAtSplinePoint` (`/Game/BluePrint/BP_QbertJumpArcSpline.Spline` (`self.JumpArcSpline`)) 2 (+ (`self.FallTileLocation`) (0.0 -2.0 -300.0)) "World" true)
  (bind (_direction _0_1) (`Timeline|Timeline_1` :!via `PlayFromStart`)
    (:`Update`
      (`self.K2_SetActorLocation` (`SplineComponent.GetLocationAtDistanceAlongSpline` (`/Game/BluePrint/BP_QbertJumpArcSpline.Spline` (`self.JumpArcSpline`)) (`KismetMathLibrary.Lerp` 0.0 (`SplineComponent.GetSplineLength` (`/Game/BluePrint/BP_QbertJumpArcSpline.Spline` (`self.JumpArcSpline`))) _0_1) "World")))
    (:`Finished`
      (`KismetSystemLibrary.Delay` 1.5)
      (`self.ResetPlayer`))))

(event `ResetPlayer`
  ;[1 1 1] Reset Player
  (`self.K2_SetActorLocation` (0.0 5.2 16.0))
  (set `self.IsMoving` false)
  (set `self.CurrentTile` (`|GetArrayItem` (`/Game/GameMode/GM_MainLevel.TilesArray` (cast `/Game/GameMode/GM_MainLevel` (`GameplayStatics.GetGameMode`) :!pure true))))
  (`/Game/GameMode/GM_MainLevel.DecreasePlayerLive` (cast `/Game/GameMode/GM_MainLevel` (`GameplayStatics.GetGameMode`) :!pure true)))

(fn `UserConstructionScript`)