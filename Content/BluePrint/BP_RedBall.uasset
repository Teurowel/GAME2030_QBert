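; Red ball enemy for a Q*bert-style game that hops down the tile grid until it falls off and is destroyed.
; Once activated, it starts a looping timer with a randomly chosen interval, each tick picking the right or down neighbour tile at random.
; Hops reshape a shared spline actor into an arc that a timeline follows.
; A missing neighbour stops the timer and triggers the fall arc; Qbert collision only prints debug text.
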(event `self.ReceiveBeginPlay`
  (`parent.ReceiveBeginPlay`))

(event `self.ReceiveTick`
  (params (DeltaSeconds :type "Float (single-precision)"))
  ;[1 1 1] Once Activated, Start Moving
  (if (`self.Activate`)
    (`/Engine/EditorBlueprintResources/StandardMacros.DoOnce` false
      (:`Completed`
        (bind _returnvalue (`KismetSystemLibrary.K2_SetTimer` null "MoveAlongSpline" (`KismetMathLibrary.RandomFloatInRange` 1.0 3.0) true))
        (set `self.MoveAlongSplineTimer` _returnvalue)))))

(event `MoveAlongSpline`
  ;[1 1 1] Randomly Select a tile Where red ball will move to
  (if (== (`KismetMathLibrary.RandomIntegerInRange` 0 1) 0)
    (`/Engine/EditorBlueprintResources/StandardMacros.IsValid` (`/Game/BluePrint/BP_Tile.RightTile` (`self.CurrentTile`))
      (:`Is Valid`
        (set `self.CurrentTile` (`/Game/BluePrint/BP_Tile.RightTile` (`self.CurrentTile`)))
        ;[1 1 1] Move along Spline
        (`self.K2_SetActorLocation` (`self.JumpArcSpline`) (`self.K2_GetActorLocation`) false false :!label _label)
        (`SplineComponent.SetLocationAtSplinePoint` (`/Game/BluePrint/BP_QbertJumpArcSpline.Spline` (`self.JumpArcSpline`)) 1 (+ (`self.K2_GetActorLocation` (`self.CurrentTile`)) (0.0 0.2 40.0)) "World" false)
        (`SplineComponent.SetLocationAtSplinePoint` (`/Game/BluePrint/BP_QbertJumpArcSpline.Spline` (`self.JumpArcSpline`)) 2 (+ (`self.K2_GetActorLocation` (`self.CurrentTile`)) (0.0 0.2 10.0)) "World" true)
        (bind (_direction _0_1) (`Timeline|Timeline_1` :!via `PlayFromStart`)
          (:`Update`
            (`self.K2_SetActorLocation` (`SplineComponent.GetLocationAtDistanceAlongSpline` (`/Game/BluePrint/BP_QbertJumpArcSpline.Spline` (`self.JumpArcSpline`)) (`KismetMathLibrary.Lerp` 0.0 (`SplineComponent.GetSplineLength` (`/Game/BluePrint/BP_QbertJumpArcSpline.Spline` (`self.JumpArcSpline`))) _0_1) "World")))))
      (:`Is Not Valid`
        (set `self.FallTileLocation` (+ (`self.K2_GetActorLocation` (`self.CurrentTile`)) (16.0 0.0 -24.0)))
        (`self.MoveAlongFallSpline`)))
    (else
      (`/Engine/EditorBlueprintResources/StandardMacros.IsValid` (`/Game/BluePrint/BP_Tile.DownTile` (`self.CurrentTile`))
        (:`Is Valid`
          (set `self.CurrentTile` (`/Game/BluePrint/BP_Tile.DownTile` (`self.CurrentTile`)))
          (goto _label))
        (:`Is Not Valid`
          (set `self.FallTileLocation` (+ (`self.K2_GetActorLocation` (`self.CurrentTile`)) (-16.0 0.0 -24.0)))
          (`self.MoveAlongFallSpline`))))))

(event `MoveAlongFallSpline`
  (`KismetSystemLibrary.K2_ClearAndInvalidateTimerHandle` (`self.MoveAlongSplineTimer`))
  ;[1 1 1] Move along Fall Spline
  (`self.K2_SetActorLocation` (`self.JumpArcSpline`) (`self.K2_GetActorLocation`) false false)
  (`SplineComponent.SetLocationAtSplinePoint` (`/Game/BluePrint/BP_QbertJumpArcSpline.Spline` (`self.JumpArcSpline`)) 1 (+ (`self.FallTileLocation`) (0.0 0.2 40.0)) "World" false)
  (`SplineComponent.SetLocationAtSplinePoint` (`/Game/BluePrint/BP_QbertJumpArcSpline.Spline` (`self.JumpArcSpline`)) 2 (+ (`self.FallTileLocation`) (0.0 0.2 -100.0)) "World" true)
  (bind (_direction _0_1) (`Timeline|Timeline_2` :!via `PlayFromStart`)
    (:`Update`
      (`self.K2_SetActorLocation` (`SplineComponent.GetLocationAtDistanceAlongSpline` (`/Game/BluePrint/BP_QbertJumpArcSpline.Spline` (`self.JumpArcSpline`)) (`KismetMathLibrary.Lerp` 0.0 (`SplineComponent.GetSplineLength` (`/Game/BluePrint/BP_QbertJumpArcSpline.Spline` (`self.JumpArcSpline`))) _0_1) "World")))
    (:`Finished`
      (`self.DestroyEnemy`))))

(event `self.CollisionWithQbert`
  (`KismetSystemLibrary.PrintString` "Hello"))

(fn `UserConstructionScript`
  (`parent.UserConstructionScript`))