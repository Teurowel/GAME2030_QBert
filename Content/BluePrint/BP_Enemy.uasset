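; BP_Enemy is a Q*bert-style enemy that makes an arcing entry jump onto its first tile when play begins.
; It spawns a BP_QbertJumpArcSpline, moves it to the enemy's location and places two spline points above CurrentTile.
; A timeline lerps distance along that spline to move the actor, then sets Activate once the jump finishes.
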(event `self.ReceiveBeginPlay`
  (bind _returnvalue (`|SpawnActorFromClass` "/Game/BluePrint/BP_QbertJumpArcSpline.BP_QbertJumpArcSpline_C" (`self.GetTransform`) "Undefined" "OverrideRootScale" null null))
  (set `self.JumpArcSpline` _returnvalue)
  (`self.StartMoveAlongSpline`))

(event `StartMoveAlongSpline`
  ;[1 1 1] Move to First Tile
  (`self.K2_SetActorLocation` (`self.JumpArcSpline`) (`self.K2_GetActorLocation`) false false)
  (`SplineComponent.SetLocationAtSplinePoint` (`/Game/BluePrint/BP_QbertJumpArcSpline.Spline` (`self.JumpArcSpline`)) 1 (+ (`self.K2_GetActorLocation` (`self.CurrentTile`)) (0.0 0.2 50.0)) "World" false)
  (`SplineComponent.SetLocationAtSplinePoint` (`/Game/BluePrint/BP_QbertJumpArcSpline.Spline` (`self.JumpArcSpline`)) 2 (+ (`self.K2_GetActorLocation` (`self.CurrentTile`)) (0.0 0.2 10.0)) "World" true)
  (bind (_direction _0_1) (`Timeline|Timeline_0` :!via `PlayFromStart`)
    (:`Update`
      (`self.K2_SetActorLocation` (`SplineComponent.GetLocationAtDistanceAlongSpline` (`/Game/BluePrint/BP_QbertJumpArcSpline.Spline` (`self.JumpArcSpline`)) (`KismetMathLibrary.Lerp` 0.0 (`SplineComponent.GetSplineLength` (`/Game/BluePrint/BP_QbertJumpArcSpline.Spline` (`self.JumpArcSpline`))) _0_1) "World")))
    (:`Finished`
      (set `self.Activate` true))))

(fn `UserConstructionScript`)